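; BP_Chest is a lootable chest that opens the loot inventory UI when the player interacts with it in range.
; On BeginPlay it seeds its Inventory with a RandomID1 entry.
; Trigger overlap toggles the prompt widget and interaction flag, and registers or clears the chest as the player character's overlapped interactable.
; Interactwith reaches the HUD's loot widget through BP_GameMode, then shows it, refreshes it and switches to UI-only input with a cursor.
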(event OnComponentBeginOverlap(TriggerCollision)
  (params (OverlappedComponent :type Primitive%20Component%20Object%20Reference) (OtherActor :type Actor%20Object%20Reference) (OtherComp :type Primitive%20Component%20Object%20Reference) (OtherBodyIndex :type Integer) (bFromSweep :type Boolean) (SweepResult :type Hit%20Result%20Structure%20%28by%20ref%29))
  (bind _returnvalue (Game|GetPlayerCharacter 0))
  (if (== OtherActor _returnvalue)
    (Rendering|SetVisibility (Variables|Default|GetWidget) true false)
    (Variables|Default|SetCanBeInteractedWith true)
    (bind _ascharacter_base (Utilities|Casting|CastToCharacter_base _returnvalue))
    (Variables|/Game/_PRE/Character/Character_base.Character_base_C|SetOverlappedInteractableObject _ascharacter_base self)))

(event OnComponentEndOverlap(TriggerCollision)
  (params (OverlappedComponent :type Primitive%20Component%20Object%20Reference) (OtherActor :type Actor%20Object%20Reference) (OtherComp :type Primitive%20Component%20Object%20Reference) (OtherBodyIndex :type Integer))
  (bind _returnvalue (Game|GetPlayerCharacter 0))
  (if (== OtherActor _returnvalue)
    (Rendering|SetVisibility (Variables|Default|GetWidget) false false)
    (Variables|Default|SetCanBeInteractedWith false)
    (bind _ascharacter_base (Utilities|Casting|CastToCharacter_base _returnvalue))
    (Variables|/Game/_PRE/Character/Character_base.Character_base_C|SetOverlappedInteractableObject _ascharacter_base 0)))

(event EventInteractwith
  (params (Player :type Character%20Base%20Object%20Reference))
  (bind _returnvalue (Game|GetPlayerController 0))
  (if (Variables|Default|GetCanBeInteractedWith)
    (bind _asbp_game_mode (Utilities|Casting|CastToBP_GameMode (Game|GetGameMode)))
    (Widget|SetVisibility (Variables|/Game/_PRE/Widget/W_HUD.W_HUD_C|GetW_LootInventory (Variables|/Game/_PRE/BP_GameMode.BP_GameMode_C|GetPlayerHUD _asbp_game_mode)) "Visible")
    (Input|SetInputModeUIOnly _returnvalue (Variables|/Game/_PRE/Widget/W_HUD.W_HUD_C|GetW_LootInventory (Variables|/Game/_PRE/BP_GameMode.BP_GameMode_C|GetPlayerHUD _asbp_game_mode)) "DoNotLock")
    (Variables|/Script/Engine.PlayerController|SetbShowMouseCursor _returnvalue true)
    (Default|UpdateLootInventory (Variables|/Game/_PRE/Widget/W_HUD.W_HUD_C|GetW_LootInventory (Variables|/Game/_PRE/BP_GameMode.BP_GameMode_C|GetPlayerHUD _asbp_game_mode)))))

(event EventBeginPlay
  (Utilities|Map|Add (Variables|Default|GetInventory) (Variables|Default|GetRandomID_1) 0))

(fn ConstructionScript)