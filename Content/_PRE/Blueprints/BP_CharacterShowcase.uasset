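; A character showcase actor that renders a rotatable copy of the player's character through a scene capture.
; StartRender copies the player's skeletal mesh and anim class, then attaches copies of both crossbow meshes at hand sockets; StopRender deactivates the capture.
; The construction script limits the capture to this actor's own components.
; Click and mouse-move events turn horizontal drag into yaw rotation of the preview mesh.
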(event Custom|MouseMove
  (params (MouseLocation :type Vector%202D%20Structure))
  (if (Variables|Default|GetCanRotate?)
    (Transformation|AddWorldRotation (Variables|Default|GetSkeletalMesh) (Math|Rotator|MakeRotator 0.0 0.0 (* (.X (Math|Vector2D|BreakVector2D (- MouseLocation (Variables|Default|GetStartLocation)))) -1.0)) false false)
    (Variables|Default|SetStartLocation MouseLocation)))

(event Custom|ClickedStart
  (params (MouseLocation :type Vector%202D%20Structure))
  (Variables|Default|SetStartLocation MouseLocation)
  (Variables|Default|SetCanRotate? true))

(event Custom|StartRender
  (bind _skeletalmesh (Variables|Default|GetSkeletalMesh))
  (bind _ascharacter_base (Utilities|Casting|CastToCharacter_base (Game|GetPlayerCharacter 0)))
  (bind _output_get (Variables|Default|SetAs%20Character%20Base _ascharacter_base))
  (bind _output_get_2 (Variables|Default|SetMesh (Variables|/Script/Engine.Character|GetMesh _output_get)))
  (Class|SkinnedMeshComponent|SetSkeletalMesh _skeletalmesh (Variables|/Script/Engine.SkinnedMeshComponent|GetSkeletalMesh _output_get_2) true)
  (Class|SkeletalMeshComponent|SetAnimClass _skeletalmesh (Utilities|GetClass (Components|SkeletalMesh|GetAnimInstance _output_get_2)))
  (Components|Activation|SetActive (Variables|Default|GetSceneCaptureComponent2D) true false)
  (CallFunction|UpdateWeapon))

(event Custom|ClickedEnd
  (Variables|Default|SetCanRotate? false))

(event Custom|StopRender
  (Components|Activation|SetActive (Variables|Default|GetSceneCaptureComponent2D) false false))

(event EventBeginPlay)

(fn ConstructionScript
  (Rendering|SceneCapture|ShowOnlyActorComponents (Variables|Default|GetSceneCaptureComponent2D) self false))

(fn UpdateWeapon
  (bind _as_character_base (Variables|Default|GetAs%20Character%20Base))
  (Class|SkinnedMeshComponent|SetSkeletalMesh (Variables|Default|GetWeaponMesh_R) (Variables|/Script/Engine.SkinnedMeshComponent|GetSkeletalMesh (Variables|/Game/_PRE/Character/Model/BP_Crossbow.BP_Crossbow_C|GetSkeletalMesh (Variables|/Game/_PRE/Character/Character_base.Character_base_C|GetCrossbow_R _as_character_base))) true)
  (Transformation|AttachComponentToComponent (Variables|Default|GetWeaponMesh_R) (Variables|Default|GetSkeletalMesh) "Crossbow_RSocket" "SnapToTarget" "SnapToTarget" "KeepWorld" true)
  (Class|SkinnedMeshComponent|SetSkeletalMesh (Variables|Default|GetWeaponMesh_L) (Variables|/Script/Engine.SkinnedMeshComponent|GetSkeletalMesh (Variables|/Game/_PRE/Character/Model/BP_Crossbow.BP_Crossbow_C|GetSkeletalMesh (Variables|/Game/_PRE/Character/Character_base.Character_base_C|GetCrossbow_L _as_character_base))) true)
  (Transformation|AttachComponentToComponent (Variables|Default|GetWeaponMesh_L) (Variables|Default|GetSkeletalMesh) "Crossbow_LSocket" "KeepRelative" "KeepRelative" "KeepWorld" true))