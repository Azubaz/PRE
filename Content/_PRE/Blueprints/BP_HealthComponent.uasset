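; Health component that tracks current health as a normalized percentage and flags death when it reaches zero.
; Damage is two-stage: RemoveHP writes a clamped result to a buffer with its own percentage, leaving current health untouched.
; UpdateHP commits the buffer to current health and recalculates the percentage and death check, which also runs on BeginPlay.
; Repeated RemoveHP calls before a commit overwrite the buffer rather than stack.
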(event EventBeginPlay
  (CallFunction|CalculatePercentage))

(fn CalculatePercentage
  (bind _output_get (Variables|Default|SetCurrentPercentage (Math|Float|NormalizetoRange (Variables|Default|GetCurrentHealth) 0.0 (Variables|Default|GetMaxHealth))))
  (if (== _output_get 0.0)
    (Variables|Default|SetIsDead? true)))

(fn RemoveHP
  (params (Amount :type Float%20%28single-precision%29))
  (Variables|Default|SetBufferHP (Math|Float|Clamp(Float) (- (Variables|Default|GetCurrentHealth) Amount) 0.0 (Variables|Default|GetMaxHealth)))
  (CallFunction|CalculatePercentageBuffer))

(fn CalculatePercentageBuffer
  (Variables|Default|SetBufferPercentage (Math|Float|NormalizetoRange (Variables|Default|GetBufferHP) 0.0 (Variables|Default|GetMaxHealth))))

(fn UpdateHP
  (Variables|Default|SetCurrentHealth (Variables|Default|GetBufferHP))
  (CallFunction|CalculatePercentage))