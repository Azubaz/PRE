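; Enemy spawner that spawns wave-based groups of enemies at spawn points supplied by BP_GameMode.
; Shortly after BeginPlay it caches three spawn point sets, registers itself and the wave count with the game mode, then runs SetupWave.
; SetupWave picks the current wave's enemy array and a point set matching its size, both limited to three options.
; Spawned actors, current wave and enemy count are written back to the game mode.
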(event Custom|SetupWave
  (bind _spawnedenemies (Variables|Default|GetSpawnedEnemies))
  (Utilities|Array|Clear (Variables|Default|GetSpawnedEnemies))
  (bind _enemyarray (CallFunction|SetEnemyArray (Variables|Default|GetCurrentWave)))
  (bind _selectedarray (CallFunction|SetSpawnArray (Utilities|Array|Length _enemyarray)))
  (for (_array_element _array_index) _selectedarray
    (bind _returnvalue (Game|SpawnActorfromClass (Utilities|Array|Get(acopy) _enemyarray _array_index) (Transformation|GetActorTransform _array_element) "Undefined" 0 0))
    (Utilities|Array|SetArrayElem (Variables|Default|GetSpawnedEnemies) _array_index _returnvalue true))
  (bind _asbp_game_mode (Utilities|Casting|CastToBP_GameMode (Game|GetGameMode)))
  (Variables|/Game/_PRE/BP_GameMode.BP_GameMode_C|SetSpawnedEnemyArray _asbp_game_mode _spawnedenemies)
  (Variables|/Game/_PRE/BP_GameMode.BP_GameMode_C|SetCurrentWave _asbp_game_mode (Variables|Default|GetCurrentWave))
  (Variables|/Game/_PRE/BP_GameMode.BP_GameMode_C|SetNumberOfEnemies _asbp_game_mode (Utilities|Array|Length _spawnedenemies)))

(event EventBeginPlay
  (Utilities|FlowControl|Delay 0.5)
  (bind _asbp_game_mode (Utilities|Casting|CastToBP_GameMode (Game|GetGameMode)))
  (Variables|Default|SetSpawn%20Point%201 (Variables|/Game/_PRE/BP_GameMode.BP_GameMode_C|GetSpawnPoint1 _asbp_game_mode))
  (Variables|Default|SetSpawn%20Point%202 (Variables|/Game/_PRE/BP_GameMode.BP_GameMode_C|GetSpawnPoint2 _asbp_game_mode))
  (Variables|Default|SetSpawn%20Point%203 (Variables|/Game/_PRE/BP_GameMode.BP_GameMode_C|GetSpawnPoint3 _asbp_game_mode))
  (Variables|/Game/_PRE/BP_GameMode.BP_GameMode_C|SetEnemySpawnerReference _asbp_game_mode self)
  (Variables|/Game/_PRE/BP_GameMode.BP_GameMode_C|SetMaxWaves _asbp_game_mode (Variables|Default|GetNumberOfWaves))
  (CallFunction|SetupWave))

(fn ConstructionScript)

(fn SetSpawnArray
  (params (ArrayLenght :type Integer))
  (if (== ArrayLenght 1)
    (return (Variables|Default|GetSpawn%20Point%201))
    (elif (== ArrayLenght 2)
      (return (Variables|Default|GetSpawn%20Point%202))
      (elif (== ArrayLenght 3)
        (return (Variables|Default|GetSpawn%20Point%203))))))

(fn SetEnemyArray
  (params (Wave :type Integer))
  (if (== Wave 1)
    (return (Variables|Default|GetEnemy%20Wave%201))
    (elif (== Wave 2)
      (return (Variables|Default|GetEnemy%20Wave%202))
      (elif (== Wave 3)
        (return (Variables|Default|GetEnemy%20Wave%203))))))