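; Game mode for wave-based levels that sets up the player HUD and runs wave progression and victory.
; On BeginPlay it waits out any level sequence, then loads the save slot's inventories and progress into the game instance before initializing the player character.
; NextWave has the enemy spawner set up each wave until the count is exceeded.
; WinGame then opens the reward chest and advances capped level progress on the game instance.
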(event Custom|NextWave
  (bind _enemyspawnerreference (Variables|Default|GetEnemySpawnerReference))
  (bind _output_get (Variables|/Game/_PRE/Blueprints/SpawnSystem/BP_EnemySpawner.BP_EnemySpawner_C|SetCurrentWave _enemyspawnerreference (+ (Variables|/Game/_PRE/Blueprints/SpawnSystem/BP_EnemySpawner.BP_EnemySpawner_C|GetCurrentWave _enemyspawnerreference) 1)))
  (if (> _output_get (Variables|/Game/_PRE/Blueprints/SpawnSystem/BP_EnemySpawner.BP_EnemySpawner_C|GetNumberOfWaves _enemyspawnerreference))
    (CallFunction|WinGame)
    (else
      (Utilities|Array|Clear (Variables|Default|GetSpawnedEnemyArray))
      (Default|SetupWave (Variables|Default|GetEnemySpawnerReference))
      (Development|PrintString (Utilities|String|ToString(Integer) (Variables|Default|GetCurrentWave))))))

(event Custom|WinGame
  (bind _chest (Variables|Default|GetChest))
  ;[1 1 1] Enable reward chest to be opened and set new material to indicate
  (Development|PrintString "You Win!")
  (Components|Animation|PlayAnimation (Variables|/Game/_PRE/Blueprints/BP_Chest.BP_Chest_C|GetSkeletalMesh _chest) "/Game/_PRE/Blueprints/mesh/Chest_Anim_Chest_OpeningAnim.Chest_Anim_Chest_OpeningAnim" false)
  (Audio|PlaySoundatLocation "/Game/_PRE/Sound_Effects/Chest_Open.Chest_Open" (Transformation|GetActorLocation _chest) "0, 0, 0" 1.0 1.0 0.0 0 0 _chest)
  (Variables|/Script/Engine.PrimitiveComponent|SetbGenerateOverlapEvents (Variables|/Game/_PRE/Blueprints/BP_Chest.BP_Chest_C|GetTriggerCollision _chest) true)
  ;[1 1 1] Save new progress if current level = next level -1
  (bind _asbp_game_instance (Utilities|Casting|CastToBP_GameInstance (Game|GetGameInstance)))
  (if (and (== (Variables|/Game/_PRE/BP_GameInstance.BP_GameInstance_C|GetCurrentLevel _asbp_game_instance) (Variables|/Game/_PRE/BP_GameInstance.BP_GameInstance_C|GetLevelProgress _asbp_game_instance)) (<= (Variables|/Game/_PRE/BP_GameInstance.BP_GameInstance_C|GetCurrentLevel _asbp_game_instance) 15))
    (Variables|/Game/_PRE/BP_GameInstance.BP_GameInstance_C|SetLevelProgress _asbp_game_instance (+ (Variables|/Game/_PRE/BP_GameInstance.BP_GameInstance_C|GetCurrentLevel _asbp_game_instance) 1))))

(event EventBeginPlay
  (bind _levelsequence (Variables|Default|GetLevelSequence))
  (Utilities|FlowControl|Delay 0.1)
  (Utilities|IsValid _levelsequence
    (:Is%20Valid
      (Utilities|FlowControl|Delay (Class|TimeManagementBlueprintLibrary|ToSeconds(QualifiedFrameTime) (Media|MediaPlayer|GetDuration (Variables|/Script/LevelSequence.LevelSequenceActor|GetSequencePlayer _levelsequence)))))
    (:Is%20Not%20Valid
      (Development|PrintString "Hello")))
  (bind _returnvalue (UserInterface|CreateWidget "/Game/_PRE/Widget/W_HUD.W_HUD_C"))
  (bind _output_get (Variables|Default|SetPlayerHUD _returnvalue))
  (UserInterface|Viewport|AddtoViewport _output_get 0)
  (Input|SetInputModeGameOnly (Game|GetPlayerController 0))
  (bind _returnvalue_2 (SaveGame|DoesSaveGameExist "SavedGameSlot"))
  (if _returnvalue_2
    (bind _returnvalue_3 (SaveGame|LoadGamefromSlot "SavedGameSlot"))
    (bind _asbp_save_game (Utilities|Casting|CastToBP_SaveGame _returnvalue_3))
    (bind _asbp_game_instance (Utilities|Casting|CastToBP_GameInstance (Game|GetGameInstance)))
    (Variables|/Game/_PRE/BP_GameInstance.BP_GameInstance_C|SetWeaponInventory _asbp_game_instance (Variables|/Game/_PRE/BP_SaveGame.BP_SaveGame_C|GetWeaponInventory _asbp_save_game))
    (Variables|/Game/_PRE/BP_GameInstance.BP_GameInstance_C|SetEquipmentInventory _asbp_game_instance (Variables|/Game/_PRE/BP_SaveGame.BP_SaveGame_C|GetEquipmentInventory _asbp_save_game))
    (Variables|/Game/_PRE/BP_GameInstance.BP_GameInstance_C|SetUpgradeMatInventory _asbp_game_instance (Variables|/Game/_PRE/BP_SaveGame.BP_SaveGame_C|GetUpgradeInventory _asbp_save_game))
    (Variables|/Game/_PRE/BP_GameInstance.BP_GameInstance_C|SetLevelProgress _asbp_game_instance (Variables|/Game/_PRE/BP_SaveGame.BP_SaveGame_C|GetLevelProgress _asbp_save_game))
    (bind _ascharacter_base (Utilities|Casting|CastToCharacter_base (Game|GetPlayerCharacter 0)))
    (Variables|/Game/_PRE/Character/Character_base.Character_base_C|SetSaveFile _ascharacter_base _asbp_save_game)
    (Default|Setup _ascharacter_base)
    (else
      (Development|PrintString "No Save file exists")
      (bind _ascharacter_base_2 (Utilities|Casting|CastToCharacter_base (Game|GetPlayerCharacter 0)))
      (Default|Setup _ascharacter_base_2))))

(fn ConstructionScript)